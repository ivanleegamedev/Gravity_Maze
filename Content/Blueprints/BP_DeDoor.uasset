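; BP_DeDoor is a door driven by a count of active pressure switches.
; Switch activated and deactivated events adjust the count and compare it to the required number.
; Meeting the threshold reverses the DeDoorActivation timeline and falling short plays it forward, the inverse of a plain activation.
; The timeline's DoorPosition output sets the door's relative Z location.
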(event `DeSwitchActivated`
  (`/Engine/EditorBlueprintResources/StandardMacros.IncrementInt` (`self.PressureSwitchesActive`)
    (:`  `
      (if (>= (`self.PressureSwitchesActive`) (`self.PressureSwitchesNeeded`))
        (bind (_direction _doorposition) (`Timeline|DeDoorActivation` :!via `Reverse` :!label _label)
          (:`Update`
            (`SceneComponent.K2_SetRelativeLocation` (`self.Door`) (`KismetMathLibrary.MakeVector` 0.0 0.0 _doorposition) false false)))
        (else
          (goto _label))))))

(event `DeSwitchDeactivated`
  (`/Engine/EditorBlueprintResources/StandardMacros.DecrementInt` (`self.PressureSwitchesActive`)
    (:`  `
      (if (>= (`self.PressureSwitchesActive`) (`self.PressureSwitchesNeeded`))
        (goto _label :!via `Reverse`)
        (else
          (goto _label))))))

(fn `UserConstructionScript`)